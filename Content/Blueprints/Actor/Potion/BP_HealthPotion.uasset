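; Health potion pickup that bobs and spins in the world and applies an instant Gameplay Effect to actors that overlap it.
; BeginPlay starts sinusoidal movement and rotation through functions defined outside this graph, and Tick applies the calculated location and rotation.
; The sphere overlap passes the other actor and effect class to ApplyEffectToTarget.
; An unconnected chain that applies the effect directly through the Ability System Component never runs.
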(event `self.ReceiveBeginPlay`
  (`self.StartSinusoidalMovement`)
  (`self.StartRotation`))

(event `self.ReceiveTick`
  (params (DeltaSeconds :type "Float (single-precision)"))
  (`self.K2_SetActorLocation` (`self.CalculatedLocation`))
  (`self.K2_SetActorRotation` (`self.CalculatedRotation`)))

(event `self.Sphere.OnComponentBeginOverlap`
  (params (OverlappedComponent :type "PrimitiveComponent Object Reference") (OtherActor :type "Actor Object Reference") (OtherComp :type "PrimitiveComponent Object Reference") (OtherBodyIndex :type Integer) (bFromSweep :type Boolean) (SweepResult :type "HitResult Structure (by ref)"))
  (`self.ApplyEffectToTarget` OtherActor (`self.InstantGameplayEfectClass`)))

(fn `UserConstructionScript`)